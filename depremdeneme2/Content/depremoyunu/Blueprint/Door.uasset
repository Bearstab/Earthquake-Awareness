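; Door Blueprint that swings open and closed, with sounds, through an Open/Close event.
; A FlipFlop alternates between playing and reversing the SmoothKapi timeline, which lerps the root's world rotation toward a 90-degree yaw offset captured at opening.
; Closing runs at twice the opening speed.
; The open sound plays at the world origin, while the close sound plays at the door's location.
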(event `Open/Close`
  (bind _smoothkapi (`self.SmoothKapi`))
  (bind _returnvalue (`SceneComponent.K2_GetComponentRotation` (`self.DefaultSceneRoot`)))
  (`/Engine/EditorBlueprintResources/StandardMacros.FlipFlop`
    (:`A`
      (set `self.BaseRotation` _returnvalue)
      (set `self.TargetRotation` (`KismetMathLibrary.MakeRotator` (.roll _returnvalue) (.pitch _returnvalue) (+ (.yaw _returnvalue) 90.0)))
      (`TimelineComponent.SetPlayRate` _smoothkapi 0.8)
      (`GameplayStatics.PlaySoundAtLocation` "/Game/depremoyunu/sesler/DoorOpen.DoorOpen" (0.0 0.0 0.0) (struct) 1.0 1.0 0.0 null null null)
      (bind (_direction _kapimovement) (`Timeline|SmoothKapi` :!label _label)
        (:`Update`
          (`SceneComponent.K2_SetWorldRotation` (`self.DefaultSceneRoot`) (`KismetMathLibrary.RLerp` (`self.BaseRotation`) (`self.TargetRotation`) _kapimovement) false false))))
    (:`B`
      (`TimelineComponent.SetPlayRate` _smoothkapi 1.6)
      (`GameplayStatics.PlaySoundAtLocation` "/Game/depremoyunu/sesler/DoorClose.DoorClose" (`SceneComponent.K2_GetComponentLocation` (`self.Door`)) (struct) 1.0 1.0 0.0 null null null)
      (goto _label :!via `Reverse`))))

(fn `UserConstructionScript`)