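; LightButton is a light actor whose LightPoint component follows the on/off state of a referenced WallSwitch.
; On BeginPlay, it casts SwitchActor to WallSwitch and sets the light's visibility from that switch's IsOn.
; The Switch function repeats the same update when called, and both paths do nothing if the cast fails.
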(event `self.ReceiveBeginPlay`
  (bind _aswall_switch (cast `/Game/depremoyunu/Blueprint/WallSwitch` (`self.SwitchActor`)))
  (`SceneComponent.SetVisibility` (`self.LightPoint`) (`/Game/depremoyunu/Blueprint/WallSwitch.IsOn` _aswall_switch) false))

(fn `Switch`
  (bind _aswall_switch (cast `/Game/depremoyunu/Blueprint/WallSwitch` (`self.SwitchActor`)))
  (`SceneComponent.SetVisibility` (`self.LightPoint`) (`/Game/depremoyunu/Blueprint/WallSwitch.IsOn` _aswall_switch) false))

(fn `UserConstructionScript`)